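; BP_NPC_Character is an NPC character that uses AI movement to head toward an actor from its Destination array.
; On BeginPlay, if State matches one enum value, it issues AI MoveTo toward the valid entry at TargetPoint.
; The immediate exec output loops through a short Delay to reissue the move without awaiting arrival.
; TargetPoint has zero added each pass, so the loop never advances to another destination.
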(event EventBeginPlay
  (if (Utilities|Enum|Equal(Enum) (Variables|Default|GetState) "NewEnumerator1")
    (Utilities|IsValid (Utilities|Array|Get(acopy) (Variables|Default|GetDestination) (Variables|Default|GetTarget%20Point)) :!label _label
      (:Is%20Valid
        (AI|AIMoveTo self "0, 0, 0" (Utilities|Array|Get(acopy) (Variables|Default|GetDestination) (Variables|Default|GetTarget%20Point)) 6e+01 true
          (:then
            (Variables|Default|SetTarget%20Point (+ (Variables|Default|GetTarget%20Point) 0))
            (Utilities|FlowControl|Delay 0.2)
            (goto _label)))))))

(fn ConstructionScript)
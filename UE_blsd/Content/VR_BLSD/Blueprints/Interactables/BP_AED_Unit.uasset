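; Grabbable AED unit for VR BLSD that deploys and stows two electrode pads.
; BeginPlay gathers every BP_AED_Plate in the level, socketing each by plate type and attaching its cable.
; Interact opens it, releasing visible, physics-driven pads constrained to the now non-simulating body by array order, not type.
; Closing hides cables and pads, re-sockets pads, reports them detached to GM_BLSD and restores body physics.
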(event OnDropped(GrabComponent)
  (Physics|SetSimulatePhysics (Variables|Default|GetStaticMesh) true))

(event EventBeginPlay
  (bind _staticmesh (Variables|Default|GetStaticMesh))
  (CallFunction|SetCollisions _staticmesh)
  (for _array_element (Components|GetChildrenComponents _staticmesh false)
    (bind _asprimitive_component (Utilities|Casting|CastToPrimitiveComponent _array_element))
    (CallFunction|SetCollisions _asprimitive_component))
  (Collision|SetCollisionProfileName (Variables|Default|GetCable_R) "PhysicsActor" true :!class /Script/Engine.PrimitiveComponent)
  (Collision|SetCollisionProfileName (Variables|Default|GetCable_L) "PhysicsActor" true :!class /Script/Engine.PrimitiveComponent)
  (bind _outactors (Actor|GetAllActorsOfClass "/Game/VR_BLSD/Blueprints/Interactables/BP_AED_Plate.BP_AED_Plate_C"))
  (bind _output_get (Variables|Default|SetPads _outactors))
  (for _array_element_2 _output_get
    (switch Utilities|FlowControl|Switch|SwitchonE_PlatePosition (Variables|/Game/VR_BLSD/Blueprints/Interactables/BP_AED_Plate.BP_AED_Plate_C|GetPlateType _array_element_2)
      (:NewEnumerator0
        (Default|AttachtoSocket _array_element_2 "Socket_Pad_R" (Variables|Default|GetStaticMesh))
        (Class|CableComponent|SetAttachEndto (Variables|Default|GetCable_R) _array_element_2 "None" "None"))
      (:NewEnumerator1
        (Default|AttachtoSocket _array_element_2 "Socket_Pad_L" (Variables|Default|GetStaticMesh))
        (Class|CableComponent|SetAttachEndto (Variables|Default|GetCable_L) _array_element_2 "None" "None")))))

(event EventInteract
  (bind _pads (Variables|Default|GetPads))
  (bind _staticmesh (Variables|Default|GetStaticMesh))
  (if (Variables|Default|GetbIsOpen)
    (Rendering|SetVisibility (Variables|Default|GetCable_L) false false)
    (Rendering|SetVisibility (Variables|Default|GetCable_R) false false)
    (for _array_element (Variables|Default|GetPads)
      (Rendering|SetVisibility (Variables|/Script/Engine.Actor|GetRootComponent _array_element) false true)
      (bind _asgm_blsd (Utilities|Casting|CastToGM_BLSD (Game|GetGameMode)))
      (Default|UpdatePlateStatus _asgm_blsd (Variables|/Game/VR_BLSD/Blueprints/Interactables/BP_AED_Plate.BP_AED_Plate_C|GetPlateType _array_element) false)
      (switch Utilities|FlowControl|Switch|SwitchonE_PlatePosition (Variables|/Game/VR_BLSD/Blueprints/Interactables/BP_AED_Plate.BP_AED_Plate_C|GetPlateType _array_element)
        (:NewEnumerator0
          (Default|AttachtoSocket _array_element "Socket_Pad_R" (Variables|Default|GetStaticMesh)))
        (:NewEnumerator1
          (Default|AttachtoSocket _array_element "Socket_Pad_L" (Variables|Default|GetStaticMesh)))))
    (Physics|SetSimulatePhysics (Variables|Default|GetStaticMesh) true)
    (Variables|Default|SetbIsOpen false)
    (else
      (Rendering|SetVisibility (Variables|Default|GetCable_L) true false)
      (Rendering|SetVisibility (Variables|Default|GetCable_R) true false)
      (for _array_element_2 (Variables|Default|GetPads)
        (CallFunction|SetCollisions (Variables|/Game/VR_BLSD/Blueprints/Interactables/BP_Grabbable.BP_Grabbable_C|GetStaticMesh _array_element_2))
        (Rendering|SetVisibility (Variables|/Script/Engine.Actor|GetRootComponent _array_element_2) true true)
        (Transformation|DetachFromComponent (Variables|/Script/Engine.Actor|GetRootComponent _array_element_2) "KeepWorld" "KeepWorld" "KeepWorld" true)
        (Physics|SetSimulatePhysics (Variables|/Game/VR_BLSD/Blueprints/Interactables/BP_Grabbable.BP_Grabbable_C|GetStaticMesh _array_element_2) true))
      (Class|PhysicsConstraintComponent|SetConstrainedComponents (Variables|Default|GetConstraint_R) _staticmesh "None" (Variables|/Game/VR_BLSD/Blueprints/Interactables/BP_Grabbable.BP_Grabbable_C|GetStaticMesh (Utilities|Array|Get(acopy) _pads)) "None")
      (Class|PhysicsConstraintComponent|SetConstrainedComponents (Variables|Default|GetConstraint_L) _staticmesh "None" (Variables|/Game/VR_BLSD/Blueprints/Interactables/BP_Grabbable.BP_Grabbable_C|GetStaticMesh (Utilities|Array|Get(acopy) _pads 1)) "None")
      (Physics|SetSimulatePhysics (Variables|Default|GetStaticMesh) false)
      (Variables|Default|SetbIsOpen true))))

(fn ConstructionScript)
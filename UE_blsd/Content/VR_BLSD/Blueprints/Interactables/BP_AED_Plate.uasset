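; VR grabbable AED electrode pad for BLSD (basic life support and defibrillation), placed on the fainted body's chest.
; On release it checks overlapping components for the drop-zone tag matching its plate type, right sternum or left apex.
; A match disables physics and collision, snaps the pad to that side's socket on BP_Omar's torso, and reports the attachment to GM_BLSD.
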(event EventBeginPlay)

(event Collision|EventActorBeginOverlap
  (params (OtherActor :type Actor%20Object%20Reference)))

(event EventTick
  (params (DeltaSeconds :type Float%20%28single-precision%29)))

(fn ConstructionScript)

(fn OnEndGrab
  (|CallParentFunction)
  (for _array_element (Class|Actor|GetOverlappingComponents)
    (switch Utilities|FlowControl|Switch|SwitchonE_PlatePosition (Variables|Default|GetPlateType)
      (:NewEnumerator0
        (if (Components|ComponentHasTag _array_element "DropZone_R")
          (bind _asgm_blsd (Utilities|Casting|CastToGM_BLSD (Game|GetGameMode)))
          (bind _asbp_omar (Utilities|Casting|CastToBP_Omar (Variables|/Game/VR_BLSD/Blueprints/Core/GM_BLSD.GM_BLSD_C|GetFaintedBody _asgm_blsd)))
          (CallFunction|AttachtoSocket self "MK_Pad_R" (Variables|/Game/MetaHumans/Omar/BP_Omar.BP_Omar_C|GetTorso _asbp_omar))
          (Default|UpdatePlateStatus _asgm_blsd (Variables|Default|GetPlateType) true)))
      (:NewEnumerator1
        (if (Components|ComponentHasTag _array_element "DropZone_L")
          (bind _asgm_blsd_2 (Utilities|Casting|CastToGM_BLSD (Game|GetGameMode)))
          (bind _asbp_omar_2 (Utilities|Casting|CastToBP_Omar (Variables|/Game/VR_BLSD/Blueprints/Core/GM_BLSD.GM_BLSD_C|GetFaintedBody _asgm_blsd_2)))
          (CallFunction|AttachtoSocket self "MK_Pad_L" (Variables|/Game/MetaHumans/Omar/BP_Omar.BP_Omar_C|GetTorso _asbp_omar_2))
          (Default|UpdatePlateStatus _asgm_blsd_2 (Variables|Default|GetPlateType) true))))))

(fn AttachtoSocket
  (params (SocketName :type Name) (SocketParent :type Scene%20Component%20Object%20Reference))
  (bind _staticmesh (Variables|Default|GetStaticMesh))
  (Physics|SetSimulatePhysics _staticmesh false)
  (Collision|SetCollisionProfileName _staticmesh "Default" true :!class /Script/Engine.PrimitiveComponent)
  (Collision|SetCollisionEnabled _staticmesh "NoCollision")
  (Transformation|AttachComponentToComponent SocketParent SocketName "SnapToTarget" "SnapToTarget" "SnapToTarget" true))
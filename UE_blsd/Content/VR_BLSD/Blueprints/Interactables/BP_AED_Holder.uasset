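; AED holder cabinet for the VR BLSD content, with an interactable door that releases the AED unit.
; On BeginPlay it finds the BP_AED_Unit in the level and attaches it to the cabinet's Socket_AED.
; Interact toggles the door through separate open and close timelines that lerp its yaw.
; When opening finishes, the AED detaches and starts simulating physics; closing does not reattach it.
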(event EventBeginPlay
  (bind _returnvalue (Actor|GetActorOfClass "/Game/VR_BLSD/Blueprints/Interactables/BP_AED_Unit.BP_AED_Unit_C"))
  (bind _output_get (Variables|Default|SetAED _returnvalue))
  (Transformation|AttachComponentToComponent _output_get (Variables|Default|GetStaticMesh) "Socket_AED" "SnapToTarget" "KeepWorld" "KeepWorld" true))

(event Collision|EventActorBeginOverlap
  (params (OtherActor :type Actor%20Object%20Reference)))

(event EventTick
  (params (DeltaSeconds :type Float%20%28single-precision%29)))

(event EventInteract
  (bind _aed (Variables|Default|GetAED))
  (if (Variables|Default|GetbIsOpen)
    (bind _holderdoorfloat (Timeline|CloseHolderDoor Play)
      (:Update
        (Transformation|SetRelativeRotation (Variables|Default|GetDoor_Cabinet1_0) (Math|Rotator|MakeRotator 0.0 0.0 (Math|Float|Lerp -5e+01 -1.8e+02 _holderdoorfloat)) false false))
      (:Finished
        (Variables|Default|SetbIsOpen false)))
    (else
      (bind _holderdoorfloat_2 (Timeline|OpenHolderDoor Play)
        (:Update
          (Transformation|SetRelativeRotation (Variables|Default|GetDoor_Cabinet1_0) (Math|Rotator|MakeRotator 0.0 0.0 (Math|Float|Lerp -1.8e+02 -5e+01 _holderdoorfloat_2)) false false))
        (:Finished
          (Transformation|DetachFromComponent (Variables|/Script/Engine.Actor|GetRootComponent _aed) "KeepWorld" "KeepWorld" "KeepWorld" true)
          (Physics|SetSimulatePhysics (Variables|/Game/VR_BLSD/Blueprints/Interactables/BP_Grabbable.BP_Grabbable_C|GetStaticMesh _aed) true)
          (Variables|Default|SetbIsOpen true))))))

(fn ConstructionScript)
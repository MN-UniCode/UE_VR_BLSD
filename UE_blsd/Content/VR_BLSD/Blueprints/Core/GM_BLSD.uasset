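; Game mode for a VR BLSD training scenario, sequencing a fainting emergency guided by a Convai AI agent.
; It caches the casualty, agent, player and AED at BeginPlay.
; Stage events fire delayed narrative triggers on the agent, resetting its conversation after later stages, and attaching both AED plates ends the experience once.
; EndMenu pauses the game and shows a spawned menu in front of the headset, or the HUD menu otherwise.
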(event Custom|UpdatePlateStatus
  (params (PlateLocation :type E_PlatePosition%20Enum :default "NewEnumerator0") (IsAttached :type Boolean))
  (bind _agentconvai (Variables|Default|GetAgentConvAi))
  (switch Utilities|FlowControl|Switch|SwitchonE_PlatePosition PlateLocation
    (:NewEnumerator0
      (Variables|Default|SetbIsPlateRAttached IsAttached))
    (:NewEnumerator1
      (Variables|Default|SetbIsPlateLAttached IsAttached)))
  (if (and (Variables|Default|GetbIsPlateRAttached) (Variables|Default|GetbIsPlateLAttached))
    (Utilities|FlowControl|DoOnce false
      (:Completed
        (Utilities|FlowControl|Delay 2.0)
        (Default|StartTrigger _agentconvai "Both AED Plates Attached")
        (Variables|Default|SetbIsGameEnded true)
        (Development|PrintString "END EXPERIENCE" true true "(R=1.000000,G=0.607843,B=0.000000,A=1.000000)" 5.0)
        (Class|ConvaiChatbotComponent|ResetConversation (Variables|/ConvAI/Core/ConvaiBaseCharacter.ConvaiBaseCharacter_C|GetConvaiChatbot _agentconvai))))))

(event Custom|Trigger%20Called%20112%20Grab%20AED
  (bind _agentconvai (Variables|Default|GetAgentConvAi))
  (bind _convaichatbot (Variables|/ConvAI/Core/ConvaiBaseCharacter.ConvaiBaseCharacter_C|GetConvaiChatbot _agentconvai))
  (Utilities|FlowControl|Delay 2.0)
  (Default|StartTrigger _agentconvai "Called 112, Grab AED")
  (Development|PrintString "112 CALLED" true true "(R=1.000000,G=0.607843,B=0.000000,A=1.000000)" 5.0)
  (Development|PrintString (Variables|/Script/Convai.ConvaiChatbotComponent|GetSessionID _convaichatbot) true true "(R=0.000000,G=0.665080,B=1.000000,A=1.000000)" 5.0)
  (Class|ConvaiChatbotComponent|ResetConversation _convaichatbot)
  (Development|PrintString (Variables|/Script/Convai.ConvaiChatbotComponent|GetSessionID (Variables|/ConvAI/Core/ConvaiBaseCharacter.ConvaiBaseCharacter_C|GetConvaiChatbot _agentconvai)) true true "(R=1.000000,G=0.000000,B=0.089263,A=1.000000)" 5.0))

(event Custom|Trigger%20User%20&%20AED%20Reached%20You
  (bind _agentconvai (Variables|Default|GetAgentConvAi))
  (Utilities|FlowControl|Delay 2.0)
  (Default|StartTrigger _agentconvai "User & AED Reached You")
  (Development|PrintString "USER WITH AED" true true "(R=1.000000,G=0.607843,B=0.000000,A=1.000000)" 5.0)
  (Class|ConvaiChatbotComponent|ResetConversation (Variables|/ConvAI/Core/ConvaiBaseCharacter.ConvaiBaseCharacter_C|GetConvaiChatbot _agentconvai)))

(event Custom|Trigger%20Someone%20Fainted
  (bind _agentconvai (Variables|Default|GetAgentConvAi))
  (Utilities|FlowControl|Delay 2.0)
  (Default|Walk _agentconvai)
  (Utilities|FlowControl|Delay 2.0)
  (Default|StartTrigger _agentconvai "Someone Fainted")
  (Development|PrintString "START EXPERIENCE" true true "(R=1.000000,G=0.607843,B=0.000000,A=1.000000)" 5.0)
  (Utilities|FlowControl|Delay 2.0)
  (Variables|Default|SetbIsGuideInPosition true))

(event Custom|End%20Menu
  (Utilities|FlowControl|Sequence
    (:then_0
      (bind _asblsd_vrpawn (Utilities|Casting|CastToBLSD_VRPawn (Variables|Default|GetPlayer)))
      (if (Class|HeadMountedDisplayFunctionLibrary|IsHeadMountedDisplayEnabled)
        (Game|SpawnActorfromClass "/Game/VR_BLSD/Blueprints/BP_BLSD_Menu.BP_BLSD_Menu_C" (Math|Transform|MakeTransform (+ (Transformation|GetWorldLocation (Variables|/Game/VRTemplate/Blueprints/VRPawn.VRPawn_C|GetCamera _asblsd_vrpawn)) (* (Math|Vector|GetForwardVector (Variables|/Game/VRTemplate/Blueprints/VRPawn.VRPawn_C|GetCamera _asblsd_vrpawn)) 2e+02)) (Transformation|GetWorldRotation (Variables|/Game/VRTemplate/Blueprints/VRPawn.VRPawn_C|GetCamera _asblsd_vrpawn))) "Undefined" "MultiplyWithRoot" 0 0)
        (else
          (Default|StartMenu (Variables|/Game/VR_BLSD/Blueprints/Characters/BLSD_VRPawn.BLSD_VRPawn_C|GetHUD _asblsd_vrpawn)))))
    (:then_1
      (Input|SetInputModeUIOnly (Game|GetPlayerController 0) 0 "DoNotLock" false)
      (Game|SetGamePaused true))))

(event EventBeginPlay
  (bind _returnvalue (Actor|GetActorOfClass "/Game/VR_BLSD/Blueprints/Characters/BP_NPC_Character.BP_NPC_Character_C"))
  (Variables|Default|SetFaintedBody _returnvalue)
  (bind _returnvalue_2 (Actor|GetActorOfClass "/ConvAI/Core/ConvaiBaseCharacter.ConvaiBaseCharacter_C"))
  (Variables|Default|SetAgentConvAi _returnvalue_2)
  (bind _returnvalue_3 (Actor|GetActorOfClass "/Game/VRTemplate/Blueprints/VRPawn.VRPawn_C"))
  (Variables|Default|SetPlayer _returnvalue_3)
  (bind _returnvalue_4 (Actor|GetActorOfClass "/Game/VR_BLSD/Blueprints/Interactables/BP_AED_Unit.BP_AED_Unit_C"))
  (Variables|Default|SetAEDUnit _returnvalue_4))

(fn ConstructionScript
  (|CallParentFunction))
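; Grabbable AED defibrillator unit that toggles open and closed on Interact to deploy or stow its two pads.
; BeginPlay takes BP_AED_Plates actors from the level, assuming two, snaps them to left/right sockets and ties cable ends to them.
; Opening shows cables and pads, detaches them as physics bodies constrained to the unit, and stops the unit simulating.
; Closing hides and re-sockets them without collision, then re-enables unit physics.
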(event EventBeginPlay
  (bind _outactors (Actor|GetAllActorsOfClass "/Game/Blueprints/Grabbable/BP_AED_Plates.BP_AED_Plates_C"))
  (bind _output_get (Variables|Default|SetPads _outactors))
  (Transformation|AttachComponentToComponent (Utilities|Array|Get(acopy) _output_get) (Variables|Default|GetStaticMesh) "Socket_Pad_L" "SnapToTarget" "SnapToTarget" "SnapToTarget" true)
  (Transformation|AttachComponentToComponent (Utilities|Array|Get(acopy) _output_get 1) (Variables|Default|GetStaticMesh) "Socket_Pad_R" "SnapToTarget" "SnapToTarget" "SnapToTarget" true)
  (Class|CableComponent|SetAttachEndto (Variables|Default|GetCable_R) (Utilities|Array|Get(acopy) _output_get 1) "None" "None")
  (Class|CableComponent|SetAttachEndto (Variables|Default|GetCable_L) (Utilities|Array|Get(acopy) _output_get) "None" "None"))

(event EventInteract
  (bind _pads (Variables|Default|GetPads))
  (bind _staticmesh (Variables|Default|GetStaticMesh))
  (if (Variables|Default|GetbIsOpen)
    (Rendering|SetVisibility (Variables|Default|GetCable_L) false false)
    (Rendering|SetVisibility (Variables|Default|GetCable_R) false false)
    (for (_array_element _array_index) (Variables|Default|GetPads)
      (Physics|SetSimulatePhysics (Variables|/Game/Blueprints/Grabbable/BP_Grabbable.BP_Grabbable_C|GetStaticMesh _array_element) false)
      (Collision|SetCollisionProfileName (Variables|/Game/Blueprints/Grabbable/BP_Grabbable.BP_Grabbable_C|GetStaticMesh _array_element) "Default" true :!class /Script/Engine.PrimitiveComponent)
      (Collision|SetCollisionEnabled (Variables|/Game/Blueprints/Grabbable/BP_Grabbable.BP_Grabbable_C|GetStaticMesh _array_element) "NoCollision")
      (Rendering|SetVisibility (Variables|/Script/Engine.Actor|GetRootComponent _array_element) false true)
      (if (== _array_index 0)
        (Transformation|AttachComponentToComponent _array_element (Variables|Default|GetStaticMesh) "Socket_Pad_L" "SnapToTarget" "SnapToTarget" "SnapToTarget" true)
        (else
          (Transformation|AttachComponentToComponent _array_element (Variables|Default|GetStaticMesh) "Socket_Pad_R" "SnapToTarget" "SnapToTarget" "SnapToTarget" true))))
    (Physics|SetSimulatePhysics (Variables|Default|GetStaticMesh) true)
    (Variables|Default|SetbIsOpen false)
    (else
      (Rendering|SetVisibility (Variables|Default|GetCable_L) true false)
      (Rendering|SetVisibility (Variables|Default|GetCable_R) true false)
      (for _array_element_2 (Variables|Default|GetPads)
        (Collision|SetCollisionProfileName (Variables|/Game/Blueprints/Grabbable/BP_Grabbable.BP_Grabbable_C|GetStaticMesh _array_element_2) "PhysicsActor" true :!class /Script/Engine.PrimitiveComponent)
        (Collision|SetCollisionEnabled (Variables|/Game/Blueprints/Grabbable/BP_Grabbable.BP_Grabbable_C|GetStaticMesh _array_element_2) "QueryAndPhysics")
        (Rendering|SetVisibility (Variables|/Script/Engine.Actor|GetRootComponent _array_element_2) true true)
        (Transformation|DetachFromComponent (Variables|/Script/Engine.Actor|GetRootComponent _array_element_2) "KeepWorld" "KeepWorld" "KeepWorld" true)
        (Physics|SetSimulatePhysics (Variables|/Game/Blueprints/Grabbable/BP_Grabbable.BP_Grabbable_C|GetStaticMesh _array_element_2) true))
      (Class|PhysicsConstraintComponent|SetConstrainedComponents (Variables|Default|GetConstraint_R) _staticmesh "None" (Variables|/Game/Blueprints/Grabbable/BP_Grabbable.BP_Grabbable_C|GetStaticMesh (Utilities|Array|Get(acopy) _pads)) "None")
      (Class|PhysicsConstraintComponent|SetConstrainedComponents (Variables|Default|GetConstraint_L) _staticmesh "None" (Variables|/Game/Blueprints/Grabbable/BP_Grabbable.BP_Grabbable_C|GetStaticMesh (Utilities|Array|Get(acopy) _pads 1)) "None")
      (Physics|SetSimulatePhysics (Variables|Default|GetStaticMesh) false)
      (Variables|Default|SetbIsOpen true))))

(fn ConstructionScript)
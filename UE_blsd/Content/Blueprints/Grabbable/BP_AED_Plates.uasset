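; Grabbable AED pad for a VR first-aid scenario that sticks to the fainted patient's chest when released over a drop zone.
; On grab end, after the parent logic, it scans overlapping components for left or right drop-zone tags.
; A match disables the mesh's physics and collision, then snap-attaches it to the matching pad socket on BP_Omar's torso, found through the VRGameMode's FaintedBody.
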(event EventBeginPlay)

(event Collision|EventActorBeginOverlap
  (params (OtherActor :type Actor%20Object%20Reference)))

(event EventTick
  (params (DeltaSeconds :type Float%20%28single-precision%29)))

(fn ConstructionScript)

(fn OnEndGrab
  (bind _staticmesh (Variables|Default|GetStaticMesh))
  (bind _staticmesh_2 (Variables|Default|GetStaticMesh))
  (|CallParentFunction)
  (for _array_element (Class|Actor|GetOverlappingComponents)
    (if (Components|ComponentHasTag _array_element "DropZone_L")
      (bind _asvrgame_mode (Utilities|Casting|CastToVRGameMode (Game|GetGameMode)))
      (bind _asbp_omar (Utilities|Casting|CastToBP_Omar (Variables|/Game/VRTemplate/Blueprints/VRGameMode.VRGameMode_C|GetFaintedBody _asvrgame_mode)))
      (Physics|SetSimulatePhysics _staticmesh false)
      (Collision|SetCollisionProfileName _staticmesh "Default" true :!class /Script/Engine.PrimitiveComponent)
      (Collision|SetCollisionEnabled _staticmesh "NoCollision")
      (Transformation|AttachComponentToComponent (Variables|/Game/MetaHumans/Omar/BP_Omar.BP_Omar_C|GetTorso _asbp_omar) "MK_Pad_L" "SnapToTarget" "SnapToTarget" "SnapToTarget" true)
      (elif (Components|ComponentHasTag _array_element "DropZone_R")
        (bind _asvrgame_mode_2 (Utilities|Casting|CastToVRGameMode (Game|GetGameMode)))
        (bind _asbp_omar_2 (Utilities|Casting|CastToBP_Omar (Variables|/Game/VRTemplate/Blueprints/VRGameMode.VRGameMode_C|GetFaintedBody _asvrgame_mode_2)))
        (Physics|SetSimulatePhysics _staticmesh_2 false)
        (Collision|SetCollisionProfileName _staticmesh_2 "Default" true :!class /Script/Engine.PrimitiveComponent)
        (Collision|SetCollisionEnabled _staticmesh_2 "NoCollision")
        (Transformation|AttachComponentToComponent (Variables|/Game/MetaHumans/Omar/BP_Omar.BP_Omar_C|GetTorso _asbp_omar_2) "MK_Pad_R" "SnapToTarget" "SnapToTarget" "SnapToTarget" true)))))
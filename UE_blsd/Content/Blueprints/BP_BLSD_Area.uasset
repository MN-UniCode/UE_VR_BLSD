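; BP_BLSD_Area is a Box trigger area for the BLSD part of a VR game, currently a stub with no gameplay effect.
; On each begin overlap it casts the game mode to VRGameMode and tests whether its Player, AgentConvAi and FaintedBody are all inside the box.
; The branch that follows this three-actor check has no actions wired to it.
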(event OnComponentBeginOverlap(Box)
  (params (OverlappedComponent :type Primitive%20Component%20Object%20Reference) (OtherActor :type Actor%20Object%20Reference) (OtherComp :type Primitive%20Component%20Object%20Reference) (OtherBodyIndex :type Integer) (bFromSweep :type Boolean) (SweepResult :type Hit%20Result%20Structure%20%28by%20ref%29))
  (bind _box (Variables|Default|GetBox))
  (bind _asvrgame_mode (Utilities|Casting|CastToVRGameMode (Game|GetGameMode)))
  (if (Math|Boolean|ANDBoolean (Collision|IsOverlappingActor _box (Variables|/Game/VRTemplate/Blueprints/VRGameMode.VRGameMode_C|GetPlayer _asvrgame_mode) :!class /Script/Engine.PrimitiveComponent) (Collision|IsOverlappingActor _box (Variables|/Game/VRTemplate/Blueprints/VRGameMode.VRGameMode_C|GetAgentConvAi _asvrgame_mode) :!class /Script/Engine.PrimitiveComponent) (Collision|IsOverlappingActor _box (Variables|/Game/VRTemplate/Blueprints/VRGameMode.VRGameMode_C|GetFaintedBody _asvrgame_mode) :!class /Script/Engine.PrimitiveComponent))
    _))

(event EventBeginPlay)

(event Collision|EventActorBeginOverlap
  (params (OtherActor :type Actor%20Object%20Reference)))

(event EventTick
  (params (DeltaSeconds :type Float%20%28single-precision%29)))

(fn ConstructionScript)